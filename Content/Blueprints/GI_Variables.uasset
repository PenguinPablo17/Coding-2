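; Game instance that manages the player's save data through an SG_Data save object in a single slot.
; On Init, it loads the existing save or creates a new object in memory.
; SavePlayerData writes the third-person character's health and capsule location to the slot, while LoadPlayerData restores only health from the cached object.
; ClearPlayerData deletes the slot but leaves the cached object untouched.
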(event `self.ReceiveInit`
  (bind _returnvalue (`GameplayStatics.DoesSaveGameExist` (`self.Save Slot`)))
  (if _returnvalue
    ;[1 1 1] Load Saved Grame
    (bind _returnvalue_2 (`GameplayStatics.LoadGameFromSlot` (`self.Save Slot`)))
    (bind _assg_data (cast `/Game/Blueprints/SG_Data` _returnvalue_2))
    (set `self.SaveGameData` _assg_data)
    (else
      ;[1 1 1] Create save game
      (bind _returnvalue_3 (`GameplayStatics.CreateSaveGameObject` "/Game/Blueprints/SG_Data.SG_Data_C"))
      (set `self.SaveGameData` _returnvalue_3))))

(fn `ClearPlayerData`
  (`GameplayStatics.DeleteGameInSlot` (`self.Save Slot`)))

(fn `LoadPlayerData`
  (bind _asbp_third_person_character (cast `/Game/ThirdPerson/Blueprints/BP_ThirdPersonCharacter` (`GameplayStatics.GetPlayerCharacter` 0)))
  (bind _output_get (set `self.PlayerRef` _asbp_third_person_character))
  (set `/Game/ThirdPerson/Blueprints/BP_ThirdPersonCharacter.Health` (`/Game/Blueprints/SG_Data.Health` (`self.SaveGameData`)) _output_get))

(fn `SavePlayerData`
  (bind _savegamedata (`self.SaveGameData`))
  (bind _asbp_third_person_character (cast `/Game/ThirdPerson/Blueprints/BP_ThirdPersonCharacter` (`GameplayStatics.GetPlayerCharacter` 0)))
  (set `/Game/Blueprints/SG_Data.Health` (`/Game/ThirdPerson/Blueprints/BP_ThirdPersonCharacter.Health` _asbp_third_person_character) _savegamedata)
  (set `/Game/Blueprints/SG_Data.Location` (`SceneComponent.K2_GetComponentLocation` (`Character.CapsuleComponent` (`GameplayStatics.GetPlayerCharacter` 0))) _savegamedata)
  (`GameplayStatics.SaveGameToSlot` (`self.SaveGameData`) (`self.Save Slot`)))