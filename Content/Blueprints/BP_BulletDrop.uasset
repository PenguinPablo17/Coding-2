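; Debug actor that simulates and visualises bullet drop from an Arrow component.
; From BeginPlay it loops every 0.2 seconds, drawing the engine's predicted projectile path with collision tracing.
; Each pass also runs a hand-written stepper that lowers Z velocity, draws lines and spheres, then resets start and velocity.
; The stepper sets each new start point to the velocity vector rather than the previous end point.
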(event `Really Cool Bullet Drop Calc`
  (set `self.End` (+ (`self.Start Location`) (/ (`self.Velocity`) (`KismetMathLibrary.MakeVector` (`self.SimFrequency`) 1.0 1.0))))
  ;[1 1 1] Bullet Drop sim from scratch?
  (for _ (range 21)
    (`KismetSystemLibrary.DrawDebugLine` (`self.Start Location`) (`self.End`) (struct :`R` 0.078226 :`G` 0.061898 :`B` 1.0 :`A` 1.0) (`self.MaxSimTime`))
    (`KismetSystemLibrary.DrawDebugSphere` (`self.End`) 10.0 12 (struct :`G` 0.084157 :`B` 1.0 :`A` 1.0) (`self.MaxSimTime`))
    (set `self.Start Location` (`self.Velocity`))
    (set `self.Velocity` (+ (`self.Velocity`) (0.0 0.0 -0.1)))
    (set `self.End` (+ (`self.Start Location`) (/ (`self.Velocity`) (`KismetMathLibrary.MakeVector` (`self.SimFrequency`) 1.0 1.0)))))
  (set `self.Start Location` (`SceneComponent.K2_GetComponentLocation` (`self.Arrow`)))
  (set `self.Velocity` (400.0 0.0 0.0)))

(event `self.ReceiveBeginPlay`
  ;[1 1 1] Bullet drop simulator
  (set `self.Start Location` (`SceneComponent.K2_GetComponentLocation` (`self.Arrow`)))
  (`GameplayStatics.Blueprint_PredictProjectilePath_Advanced` (make `PredictProjectilePathParams` (`self.Start Location`) (`self.Velocity`) true 0.0 (`self.MaxSimTime`) true "ECC_WorldStatic" _ _ (`self.SimFrequency`) 0.0 "ForDuration") :!label _label)
  (`KismetSystemLibrary.Delay` 0.2)
  (`|ExecutionSequence`
    (:`then_0`
      (`self.Really Cool Bullet Drop Calc`))
    (:`then_1`
      (goto _label))))

(fn `UserConstructionScript`)