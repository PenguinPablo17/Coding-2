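; BP_Door is a one-way door that opens by snapping its cube 200 units down when the first player's character overlaps its collision box.
; Opening sets IsOpened and reports the door to BP_GameState through CallDoorOpened.
; BeginPlay and the Updatedoor event reapply the open state, including that report, whenever IsOpened is already true.
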(event `Update door`
  (if (`self.IsOpened?`) :!label _label
    (`SceneComponent.K2_SetRelativeLocation` (`self.Cube`) (0.0 0.0 -200.0) false false :!label _label_2)
    (set `self.IsOpened?` true)
    (bind _asbp_game_state (cast `/Game/Blueprints/BP_GameState` (`GameplayStatics.GetGameState`)))
    (`/Game/Blueprints/BP_GameState.DoorOpened` _asbp_game_state self)))

(event `self.ReceiveBeginPlay`
  (goto _label))

(event `self.Box Collison.OnComponentBeginOverlap`
  (params (OverlappedComponent :type "PrimitiveComponent Object Reference") (OtherActor :type "Actor Object Reference") (OtherComp :type "PrimitiveComponent Object Reference") (OtherBodyIndex :type Integer) (bFromSweep :type Boolean) (SweepResult :type "HitResult Structure (by ref)"))
  (if (and (== OtherActor (`GameplayStatics.GetPlayerCharacter` 0)) (not (`self.IsOpened?`)))
    (goto _label_2)))

(fn `UserConstructionScript`)