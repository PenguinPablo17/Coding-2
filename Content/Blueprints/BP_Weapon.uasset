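; BP_Weapon is a weapon actor that randomizes its type, look and damage on construction.
; The construction script picks one of four DT_Weapons rows at random and applies its mesh to StaticObject.
; A dynamic M_Weapons material gets its Diffusion color from the row's element (Earth, Fire, Water or Lightning).
; Damage rolls between the row's base value and double that, so every construction rerun rerolls the weapon.
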(fn `Damage Setter`
  (params (`Base Damage` :type "Float (double-precision)"))
  (set `self.Damage` (`KismetMathLibrary.RandomFloatInRange` `Base Damage` (* `Base Damage` 2.0)))
  (return))

(fn `Element Select`
  (params (Element :type "/Game/Blueprints/E_DamageType Enum" :default "NewEnumerator0"))
  (returns (Color :type "LinearColor Structure"))
  (switch `/Game/Blueprints/E_DamageType` Element
    (:`NewEnumerator0`
      (return (struct :`R` 0.114413 :`G` 1.0 :`B` 0.199232 :`A` 1.0)))
    (:`NewEnumerator1`
      (return (struct :`R` 1.0 :`B` 0.052879 :`A` 1.0)))
    (:`NewEnumerator2`
      (return (struct :`R` 0.001967 :`G` 0.014586 :`B` 1.0 :`A` 1.0)))
    (:`NewEnumerator3`
      (return (struct :`R` 1.0 :`G` 0.453226 :`A` 1.0)))))

(fn `UserConstructionScript`
  (bind _static_object (`self.Static Object`))
  (bind _returnvalue (`|GetDataTableRow` "/Game/Blueprints/DT_Weapons.DT_Weapons" (`KismetStringLibrary.Conv_StringToName` (`KismetStringLibrary.Conv_IntToString` (`KismetMathLibrary.RandomIntegerInRange` 1 4))))
    (:`then`
      (bind (_model _type _element _damage) (break `/Game/Blueprints/S_Weapons` _returnvalue))
      (`StaticMeshComponent.SetStaticMesh` _static_object _model)
      (bind _returnvalue_2 (`PrimitiveComponent.CreateDynamicMaterialInstance` _static_object 0 "/Game/Blueprints/M_Weapons.M_Weapons" "None"))
      (bind _color (`self.Element Select` _element))
      (`MaterialInstanceDynamic.SetVectorParameterValue` _returnvalue_2 "Diffusion" _color)
      (`self.Damage Setter` _damage))))